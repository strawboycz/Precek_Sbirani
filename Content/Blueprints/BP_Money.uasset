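; BP_Money is a spinning money pickup that adds points on overlap.
; Tick sets yaw from game time for a constant spin.
; Overlap checks that player 0 is BP_ThirdPersonCharacter rather than checking the overlapping actor, so any overlapping actor can trigger it.
; It then destroys itself, adds a fixed amount to Points on BP_ThirdPersonGameMode, and prints the new total.
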(event Collision|EventActorBeginOverlap
  (params (OtherActor :type Actor%20Object%20Reference))
  (Utilities|Casting|CastToBP_ThirdPersonCharacter (Game|GetPlayerCharacter 0))
  (Actor|DestroyActor)
  (bind _asbp_third_person_game_mode (Utilities|Casting|CastToBP_ThirdPersonGameMode (Game|GetGameMode)))
  (bind _output_get (Variables|/Game/ThirdPerson/Blueprints/BP_ThirdPersonGameMode.BP_ThirdPersonGameMode_C|SetPoints _asbp_third_person_game_mode (+ (Variables|/Game/ThirdPerson/Blueprints/BP_ThirdPersonGameMode.BP_ThirdPersonGameMode_C|GetPoints _asbp_third_person_game_mode) 5)))
  (Development|PrintString (Utilities|String|Append "Current Points:" (Utilities|String|ToString(Integer) _output_get))))

(event EventTick
  (params (DeltaSeconds :type Float%20%28single-precision%29))
  (Transformation|SetActorRotation (Math|Rotator|MakeRotator 0.0 0.0 (* (Utilities|Time|GetGameTimeinSeconds) 1e+02))))

(fn ConstructionScript)