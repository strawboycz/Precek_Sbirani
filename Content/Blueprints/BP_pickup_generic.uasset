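; Generic pickup actor that spins in place and awards points to the player when collected.
; Tick sets its yaw from elapsed game time scaled by a rotation factor.
; The PickUp event adds the given value to the Points in BP_ThirdPersonGameMode, prints the new total and destroys the actor after a short delay.
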(event EventBeginPlay)

(event EventTick
  (params (DeltaSeconds :type Float%20%28single-precision%29))
  (Transformation|SetActorRotation (Math|Rotator|MakeRotator 0.0 0.0 (* (Utilities|Time|GetGameTimeinSeconds) (Variables|Default|GetStaticRotationFactor)))))

(event EventPickUp
  (params (PointIncrementValue :type Integer))
  (bind _asbp_third_person_game_mode (Utilities|Casting|CastToBP_ThirdPersonGameMode (Game|GetGameMode)))
  (bind _output_get (Variables|/Game/ThirdPerson/Blueprints/BP_ThirdPersonGameMode.BP_ThirdPersonGameMode_C|SetPoints _asbp_third_person_game_mode (+ (stale _output_get) PointIncrementValue)))
  (Development|PrintString (Utilities|String|Append "Current Points:" (Utilities|String|ToString(Integer) _output_get)))
  (Utilities|FlowControl|Delay 0.2)
  (Actor|DestroyActor))

(fn ConstructionScript)